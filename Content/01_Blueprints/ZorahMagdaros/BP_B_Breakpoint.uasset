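; BP_B_Breakpoint is a damageable body part for the Zorah Magdaros encounter that reacts only to Ballista hits.
; The construction script sets its type from the head, back or weakpoint flags, in that priority.
; Hits subtract hit points: head and back parts destroy themselves at zero, while weakpoints take amplified damage and are never destroyed.
; Head stun and back magma reduction are only placeholder print messages.
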(event `self.OnHit`
  (params (DamageAmount :type "Float (double-precision)") (DamageSource :type String))
  (if (`KismetStringLibrary.EqualEqual_StrStr` DamageSource "Ballista")
    (switch `int` (`self.Type`)
      (:`0`
        (`KismetSystemLibrary.PrintString` "get stunned, lol")
        (`self.ReceiveDamage` DamageAmount))
      (:`1`
        (`KismetSystemLibrary.PrintString` "less magma, yippeeeeeeeeeeeeeeeeeeee")
        (`self.ReceiveDamage` DamageAmount))
      (:`2`
        (`self.ReceiveDamage` (* DamageAmount 1.45))))))

(fn `UserConstructionScript`
  (if (`self.IsHead`)
    (set `self.Type` 0)
    (elif (`self.IsBack`)
      (set `self.Type` 1)
      (elif (`self.IsWeakpoint`)
        (set `self.Type` 2)))))